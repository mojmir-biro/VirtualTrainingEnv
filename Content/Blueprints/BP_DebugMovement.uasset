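; BP_DebugMovement is a debug helper that nudges a CapturePerformer actor around the world with the keyboard.
; Each W, A, S or D press builds a fixed horizontal world-space offset and passes it to MoveDirectional.
; MoveDirectional looks up the CapturePerformer via GetActorOfClass on every call and applies a swept world offset, giving one discrete step per press rather than continuous movement.
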(event EventBeginPlay)

(event Collision|EventActorBeginOverlap
  (params (OtherActor :type Actor%20Object%20Reference)))

(event EventTick
  (params (DeltaSeconds :type Float%20%28single-precision%29)))

(event Input|KeyboardEvents|W
  (params (Key :type Key%20Structure :default "None"))
  (:Pressed
    (Variables|Default|SetDirection (Math|Vector|MakeVector 0.0 5e+01 0.0))
    (CallFunction|MoveDirectional (Variables|Default|GetDirection))))

(event Input|KeyboardEvents|A
  (params (Key :type Key%20Structure :default "None"))
  (:Pressed
    (Variables|Default|SetDirection (Math|Vector|MakeVector 5e+01 0.0 0.0))
    (CallFunction|MoveDirectional (Variables|Default|GetDirection))))

(event Input|KeyboardEvents|S
  (params (Key :type Key%20Structure :default "None"))
  (:Pressed
    (Variables|Default|SetDirection (Math|Vector|MakeVector 0.0 -5e+01 0.0))
    (CallFunction|MoveDirectional (Variables|Default|GetDirection))))

(event Input|KeyboardEvents|D
  (params (Key :type Key%20Structure :default "None"))
  (:Pressed
    (Variables|Default|SetDirection (Math|Vector|MakeVector -5e+01 0.0 0.0))
    (CallFunction|MoveDirectional (Variables|Default|GetDirection))))

(fn ConstructionScript)

(fn MoveDirectional
  (params (Direction :type Vector))
  (bind _returnvalue (Actor|GetActorOfClass "/Script/PerformanceCaptureCore.CapturePerformer"))
  (Transformation|AddActorWorldOffset _returnvalue Direction true))