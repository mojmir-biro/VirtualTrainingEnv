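; Manager actor that runs a target training session, tracking score and health, showing win or game-over widgets and updating BP_StatDisplay.
; Tick spawns BP_Target on a random timer from one of four sides, with a random limb and difficulty-scaled speed.
; Evasion mode aims targets at BP_TorsoCollider's position at spawn time instead of a fixed point.
; Keys start or stop training and, only while stopped, switch mode or difficulty.
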(event Custom|ShowGameOver
  (bind _returnvalue (UserInterface|CreateWidget "/Game/Blueprints/WB_GameOver.WB_GameOver_C"))
  (UserInterface|Viewport|AddtoViewport _returnvalue 0)
  (Utilities|FlowControl|Delay 5.0)
  (Widget|RemovefromParent _returnvalue))

(event Custom|ShowGameWin
  (bind _returnvalue (UserInterface|CreateWidget "/Game/Blueprints/WB_GameWin.WB_GameWin_C"))
  (UserInterface|Viewport|AddtoViewport _returnvalue 0)
  (Utilities|FlowControl|Delay 5.0)
  (Widget|RemovefromParent _returnvalue))

(event EventBeginPlay
  (CallFunction|EndTraining)
  (CallFunction|UpdateDisplay))

(event Collision|EventActorBeginOverlap
  (params (OtherActor :type Actor%20Object%20Reference)))

(event EventTick
  (params (DeltaSeconds :type Float%20%28single-precision%29))
  (if (Variables|Default|GetIsRunning)
    (if (<= (Variables|Default|GetTimeToSpawn) 0.0)
      (CallFunction|SpawnTarget)
      (Variables|Default|SetTimeToSpawn (Math|Random|RandomFloatinRange 3.0 5.0))
      (else
        (Variables|Default|SetTimeToSpawn (- (Variables|Default|GetTimeToSpawn) DeltaSeconds))))))

(event Input|KeyboardEvents|SpaceBar
  (params (Key :type Key%20Structure :default "None"))
  (:Pressed
    (CallFunction|StartStopTraining)))

(event Input|KeyboardEvents|Backspace
  (params (Key :type Key%20Structure :default "None"))
  (:Pressed
    (CallFunction|ChangeMode)))

(event Input|KeyboardEvents|P
  (params (Key :type Key%20Structure :default "None"))
  (:Pressed
    (CallFunction|CycleSpeedDifficulty)))

(fn ConstructionScript)

(fn InitSettings)

(fn SpawnTarget
  (bind _returnvalue (Math|Float|MakeLiteralFloat 0.5))
  (bind _returnvalue_2 (Math|Float|MakeLiteralFloat 2e+02))
  (bind _returnvalue_3 (Math|Vector|MakeVector _returnvalue _returnvalue _returnvalue))
  (switch int (Math|Random|RandomInteger 4)
    (:0
      (LocalVariables|Setv_limb "NewEnumerator0"))
    (:1
      (LocalVariables|Setv_limb "NewEnumerator1"))
    (:2
      (LocalVariables|Setv_limb "NewEnumerator2"))
    (:3
      (LocalVariables|Setv_limb "NewEnumerator3")))
  (switch int (Math|Random|RandomInteger 4)
    (:0
      (LocalVariables|Setv_direction "NewEnumerator0")
      (LocalVariables|Setv_transform (Math|Transform|MakeTransform "0.000000,800.000000,200.000000" "0, 0, 0" _returnvalue_3)))
    (:1
      (LocalVariables|Setv_direction "NewEnumerator1")
      (LocalVariables|Setv_transform (Math|Transform|MakeTransform "0.000000,-800.000000,200.000000" "0, 0, 0" _returnvalue_3)))
    (:2
      (LocalVariables|Setv_direction "NewEnumerator2")
      (LocalVariables|Setv_transform (Math|Transform|MakeTransform "800.000000,0.000000,200.000000" "0, 0, 0" _returnvalue_3)))
    (:3
      (LocalVariables|Setv_direction "NewEnumerator3")
      (LocalVariables|Setv_transform (Math|Transform|MakeTransform "-800.000000,0.000000,200.000000" "0, 0, 0" _returnvalue_3))))
  (switch Utilities|FlowControl|Switch|SwitchonEnum_Difficulty (Variables|Default|GetSpeedDifficulty)
    (:NewEnumerator0
      (LocalVariables|Setv_speed (* _returnvalue_2 (Math|Float|MakeLiteralFloat 1.0))))
    (:NewEnumerator1
      (LocalVariables|Setv_speed (* _returnvalue_2 (Math|Float|MakeLiteralFloat 2.0))))
    (:NewEnumerator2
      (LocalVariables|Setv_speed (* _returnvalue_2 (Math|Float|MakeLiteralFloat 3.0)))))
  (if (Variables|Default|GetEvasionTraining)
    (bind _returnvalue_4 (Actor|GetActorOfClass "/Game/Blueprints/BP_TorsoCollider.BP_TorsoCollider_C"))
    (LocalVariables|Setv_targetPos (Transformation|GetActorLocation _returnvalue_4))
    (else
      (LocalVariables|Setv_targetPos "0.000000,0.000000,200.000000")))
  (Game|SpawnActorfromClass "/Game/Blueprints/BP_Target.BP_Target_C" (LocalVariables|Getv_transform) "Undefined" "MultiplyWithRoot" 0 (LocalVariables|Getv_speed) (LocalVariables|Getv_direction) (LocalVariables|Getv_targetPos) (LocalVariables|Getv_limb) 0)
  (Audio|PlaySoundatLocation "/Game/Import/Sounds/target_spawn_sound.target_spawn_sound" (.Location (Math|Transform|BreakTransform (LocalVariables|Getv_transform))) "0, 0, 0" 1.0 1.0 0.0 "/Game/Blueprints/SA_target_spawn.SA_target_spawn" 0 0 0))

(fn IncrementScore
  (bind _result (Math|Integer|IncrementInt (Variables|Default|GetScore))
    (:%20%20
      (CallFunction|UpdateDisplay)
      (if (>= _result 5)
        (CallFunction|ShowGameWin)
        (CallFunction|EndTraining))
      (return _result))))

(fn TakeDamage
  (params (HitPoints :type Integer))
  (bind _output_get (Variables|Default|SetHealth (- (Variables|Default|GetHealth) HitPoints)))
  (if (<= _output_get 0)
    (CallFunction|ShowGameOver)
    (CallFunction|EndTraining)
    (return true)
    (else
      (CallFunction|UpdateDisplay)
      (return false))))

(fn EndTraining
  (Variables|Default|SetIsRunning false)
  (Variables|Default|SetTimeToSpawn 5.0)
  (Variables|Default|SetHealth 15)
  (Variables|Default|SetScore 0)
  (bind _outactors (Actor|GetAllActorsOfClass "/Game/Blueprints/BP_Target.BP_Target_C"))
  (for _array_element _outactors
    (Actor|DestroyActor _array_element))
  (CallFunction|UpdateDisplay))

(fn BeginTraining
  (Variables|Default|SetIsRunning true)
  (CallFunction|UpdateDisplay))

(fn UpdateDisplay
  (bind _returnvalue (Actor|GetActorOfClass "/Game/Blueprints/BP_StatDisplay.BP_StatDisplay_C"))
  (Default|UpdateHealth _returnvalue (Variables|Default|GetHealth))
  (Default|UpdateScore _returnvalue (Variables|Default|GetScore))
  (Default|UpdateStatus _returnvalue (Variables|Default|GetIsRunning))
  (Default|UpdateMode _returnvalue (Variables|Default|GetEvasionTraining) (Variables|Default|GetSpeedDifficulty)))

(fn ChangeMode
  (if (not (Variables|Default|GetIsRunning))
    (Variables|Default|SetEvasionTraining (not (Variables|Default|GetEvasionTraining)))
    (CallFunction|UpdateDisplay)))

(fn StartStopTraining
  (if (Variables|Default|GetIsRunning)
    (CallFunction|EndTraining)
    (else
      (CallFunction|BeginTraining))))

(fn CycleSpeedDifficulty
  (if (not (Variables|Default|GetIsRunning))
    (switch Utilities|FlowControl|Switch|SwitchonEnum_Difficulty (Variables|Default|GetSpeedDifficulty)
      (:NewEnumerator0
        (Variables|Default|SetSpeedDifficulty "NewEnumerator1"))
      (:NewEnumerator1
        (Variables|Default|SetSpeedDifficulty "NewEnumerator2"))
      (:NewEnumerator2
        (Variables|Default|SetSpeedDifficulty "NewEnumerator0")))
    (CallFunction|UpdateDisplay)))