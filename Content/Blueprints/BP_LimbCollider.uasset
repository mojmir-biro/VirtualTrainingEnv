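; BP_LimbCollider is a limb-tagged collider that resolves overlaps with BP_Target actors in a limb-matching training game.
; The construction script colors its sphere by LimbPlacement.
; A matching limb outside evasion training bursts particles, increments the score through BP_TargetManager, updates BP_StatDisplay and destroys the target.
; Mismatches and evasion-training hits call TakeDamage on the manager, destroying the target only when it returns false.
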(event EventBeginPlay)

(event Collision|EventActorBeginOverlap
  (params (OtherActor :type Actor%20Object%20Reference))
  (bind _asbp_target (Utilities|Casting|CastToBP_Target OtherActor))
  (if (Utilities|Enum|Equal(Enum) (Utilities|String|EnumtoString (Variables|/Game/Blueprints/BP_Target.BP_Target_C|GetLimb _asbp_target)) (Utilities|String|EnumtoString (Variables|Default|GetLimbPlacement)))
    (bind _returnvalue (Actor|GetActorOfClass "/Game/Blueprints/BP_TargetManager.BP_TargetManager_C"))
    (if (Variables|/Game/Blueprints/BP_TargetManager.BP_TargetManager_C|GetEvasionTraining _returnvalue)
      (bind _hitpointzero (Default|TakeDamage (stale _returnvalue_3) 1 :!label _label))
      (if (not _hitpointzero)
        (Actor|DestroyActor _asbp_target :!label _label_2))
      (else
        (Niagara|SpawnSystematLocation "/Game/Blueprints/NS_BurstParticles.NS_BurstParticles" (Transformation|GetActorLocation _asbp_target))
        (bind _newscore (Default|IncrementScore _returnvalue))
        (bind _returnvalue_2 (Actor|GetActorOfClass "/Game/Blueprints/BP_StatDisplay.BP_StatDisplay_C"))
        (Default|UpdateScore _returnvalue_2 _newscore)
        (goto _label_2)))
    (else
      (bind _returnvalue_3 (Actor|GetActorOfClass "/Game/Blueprints/BP_TargetManager.BP_TargetManager_C"))
      (goto _label))))

(event EventTick
  (params (DeltaSeconds :type Float%20%28single-precision%29)))

(fn ConstructionScript
  (bind _sphere (Variables|Default|GetSphere))
  (switch Utilities|FlowControl|Switch|SwitchonEnum_Limbs (Variables|Default|GetLimbPlacement)
    (:NewEnumerator0
      (Rendering|Material|SetMaterial _sphere 0 "/Game/Materials/M_Target_AR.M_Target_AR"))
    (:NewEnumerator1
      (Rendering|Material|SetMaterial _sphere 0 "/Game/Materials/M_Target_AL.M_Target_AL"))
    (:NewEnumerator2
      (Rendering|Material|SetMaterial _sphere 0 "/Game/Materials/M_Target_LR.M_Target_LR"))
    (:NewEnumerator3
      (Rendering|Material|SetMaterial _sphere 0 "/Game/Materials/M_Target_LL.M_Target_LL"))))