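; BP_Target is a moving sphere target tagged with a limb, whose material is set at construction to match that arm or leg.
; Each tick it moves straight toward TargetPosition at Speed using a swept offset, then destroys itself once within a small radius.
; On arrival during evasion training, it increments the BP_TargetManager score and spawns a Niagara burst.
; An older direction-based Move function remains but is not called here.
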(event EventBeginPlay)

(event Collision|EventActorBeginOverlap
  (params (OtherActor :type Actor%20Object%20Reference)))

(event EventTick
  (params (DeltaSeconds :type Float%20%28single-precision%29))
  (bind _destroyed (CallFunction|TryDestroy))
  (if (not _destroyed)
    (CallFunction|MoveV2 DeltaSeconds)
    (else
      (Actor|DestroyActor))))

(fn ConstructionScript
  (CallFunction|InitMaterial (Variables|Default|GetLimb)))

(fn InitMaterial
  (params (p_limb :type Enum_Limbs%20Enum :default "NewEnumerator0"))
  (bind _sphere (Variables|Default|GetSphere))
  (switch Utilities|FlowControl|Switch|SwitchonEnum_Limbs p_limb
    (:NewEnumerator0
      (Rendering|Material|SetMaterial _sphere 0 "/Game/Materials/M_Target_AR.M_Target_AR"))
    (:NewEnumerator1
      (Rendering|Material|SetMaterial _sphere 0 "/Game/Materials/M_Target_AL.M_Target_AL"))
    (:NewEnumerator2
      (Rendering|Material|SetMaterial _sphere 0 "/Game/Materials/M_Target_LR.M_Target_LR"))
    (:NewEnumerator3
      (Rendering|Material|SetMaterial _sphere 0 "/Game/Materials/M_Target_LL.M_Target_LL"))))

(fn Move
  (params (p_delta :type Float%20%28double-precision%29))
  (bind _speed (Variables|Default|GetSpeed))
  (bind _returnvalue (* p_delta _speed))
  (bind _returnvalue_2 (* _returnvalue -1.0))
  (switch Utilities|FlowControl|Switch|SwitchonEnum_Direction (Variables|Default|GetDirection)
    (:NewEnumerator0
      (LocalVariables|SetOffset (Math|Vector|MakeVector 0.0 _returnvalue_2 0.0)))
    (:NewEnumerator1
      (LocalVariables|SetOffset (Math|Vector|MakeVector 0.0 _returnvalue 0.0)))
    (:NewEnumerator2
      (LocalVariables|SetOffset (Math|Vector|MakeVector _returnvalue_2 0.0 0.0)))
    (:NewEnumerator3
      (LocalVariables|SetOffset (Math|Vector|MakeVector _returnvalue 0.0 0.0))))
  (Transformation|SetActorRelativeLocation (+ (Transformation|GetActorLocation) (LocalVariables|GetOffset)) true))

(fn TryDestroy
  (bind _returnvalue (Transformation|GetActorLocation))
  (if (<= (Math|Vector|Distance(Vector) (Variables|Default|GetTargetPosition) _returnvalue) 5.0)
    (bind _returnvalue_2 (Actor|GetActorOfClass "/Game/Blueprints/BP_TargetManager.BP_TargetManager_C"))
    (if (Variables|/Game/Blueprints/BP_TargetManager.BP_TargetManager_C|GetEvasionTraining _returnvalue_2)
      (Default|IncrementScore _returnvalue_2)
      (Niagara|SpawnSystematLocation "/Game/Blueprints/NS_BurstParticles.NS_BurstParticles" _returnvalue))
    (return true)
    (else
      (return false))))

(fn MoveV2
  (params (DeltaTime :type Float%20%28double-precision%29))
  (Transformation|AddActorWorldOffset (* (Math|Vector|GetUnitDirection(Vector) (Transformation|GetActorLocation) (Variables|Default|GetTargetPosition)) (* DeltaTime (Variables|Default|GetSpeed))) true))