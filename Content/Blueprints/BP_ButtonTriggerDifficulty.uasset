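; BP_ButtonTriggerDifficulty is a button trigger that cycles the speed difficulty of the target manager.
; SetText labels the button "Diff", and ButtonAction looks up BP_TargetManager by class and calls CycleSpeedDifficulty on it.
; It has no active event logic of its own, and its construction script only calls the parent.
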(event EventBeginPlay
  (|CallParentFunction) ; This node is disabled and will not be called.\nDrag off pins to build functionality.
)

(event Collision|EventActorBeginOverlap
  (params (OtherActor :type Actor%20Object%20Reference))
  (|CallParentFunction OtherActor) ; This node is disabled and will not be called.\nDrag off pins to build functionality.
)

(event EventTick
  (params (DeltaSeconds :type Float%20%28single-precision%29))
  (|CallParentFunction DeltaSeconds) ; This node is disabled and will not be called.\nDrag off pins to build functionality.
)

(fn ConstructionScript
  (|CallParentFunction))

(fn SetText
  (Rendering|Components|TextRender|SetText (Variables|Default|GetButtonText) (Utilities|Text|MakeLiteralText "Diff")))

(fn ButtonAction
  (bind _returnvalue (Actor|GetActorOfClass "/Game/Blueprints/BP_TargetManager.BP_TargetManager_C"))
  (Default|CycleSpeedDifficulty _returnvalue))