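; BP_StatDisplay is an actor that displays game stats as text: health, score, running status and current mode.
; Four update functions take values from a caller and each write to their own text element, with no Tick or BeginPlay logic.
; Health and score are shown with labels, status toggles between "Running" and a dash, and mode combines Evasion or Target with the difficulty enum name.
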(event EventBeginPlay)

(event Collision|EventActorBeginOverlap
  (params (OtherActor :type Actor%20Object%20Reference)))

(event EventTick
  (params (DeltaSeconds :type Float%20%28single-precision%29)))

(fn ConstructionScript)

(fn UpdateHealth
  (params (NewHealth :type Integer))
  (Rendering|Components|TextRender|SetText (Variables|Default|GetHealthText) (Utilities|Text|ToText(String) (Utilities|String|Append (Utilities|String|MakeLiteralString "Health: ") (Utilities|String|ToString(Integer) NewHealth)))))

(fn UpdateScore
  (params (NewScore :type Integer))
  (Rendering|Components|TextRender|SetText (Variables|Default|GetScoreText) (Utilities|Text|ToText(String) (Utilities|String|Append (Utilities|String|MakeLiteralString "Score: ") (Utilities|String|ToString(Integer) NewScore)))))

(fn UpdateStatus
  (params (IsRunning :type Boolean))
  (bind _statustext (Variables|Default|GetStatusText))
  (if IsRunning
    (Rendering|Components|TextRender|SetText _statustext (Utilities|Text|MakeLiteralText "Running"))
    (else
      (Rendering|Components|TextRender|SetText _statustext (Utilities|Text|MakeLiteralText "-")))))

(fn UpdateMode
  (params (EvasionMode :type Boolean) (Difficulty :type Enum_Difficulty%20Enum :default "NewEnumerator0"))
  (bind _modetext (Variables|Default|GetModeText))
  (if EvasionMode
    (Rendering|Components|TextRender|SetText _modetext (Utilities|Text|ToText(String) (Utilities|String|Append (Utilities|String|MakeLiteralString "Evasion -") (Utilities|String|EnumtoString Difficulty))))
    (else
      (Rendering|Components|TextRender|SetText _modetext (Utilities|Text|ToText(String) (Utilities|String|Append (Utilities|String|MakeLiteralString "Target -") (Utilities|String|EnumtoString Difficulty)))))))